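; BP_FloorTrap is a floor trap that gives way when the player touches it, built on what appears to be a Geometry Collection component.
; Gravity on the component is switched off at BeginPlay.
; When a Player_Nick actor begins overlapping it, the component enables physics simulation and gravity, and prints a debug "Hello".
; The Chaos break event is empty, and the collision-ignore and wake-bodies calls are left unwired.
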(event `self.ReceiveBeginPlay`
  (`PrimitiveComponent.SetEnableGravity` (`self.GC_BP_FloorTrap`) false))

(event `self.GC_BP_FloorTrap.OnComponentBeginOverlap`
  (params (OverlappedComponent :type "PrimitiveComponent Object Reference") (OtherActor :type "Actor Object Reference") (OtherComp :type "PrimitiveComponent Object Reference") (OtherBodyIndex :type Integer) (bFromSweep :type Boolean) (SweepResult :type "HitResult Structure (by ref)"))
  (bind _gc_bp_floortrap (`self.GC_BP_FloorTrap`))
  (if (`GameplayStatics.ObjectIsA` OtherActor "/Script/SneakyBusiness.Player_Nick")
    (`KismetSystemLibrary.PrintString` "Hello")
    (`PrimitiveComponent.SetSimulatePhysics` _gc_bp_floortrap true)
    (`PrimitiveComponent.SetEnableGravity` _gc_bp_floortrap true)))

(event `self.GC_BP_FloorTrap.OnChaosBreakEvent`
  (params (BreakEvent :type "ChaosBreakEvent Structure (by ref)")))

(fn `UserConstructionScript`)