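; Lever Blueprint that swings between two roll angles when LeverAnim is triggered, then returns automatically.
; A timeline lerps the Root's relative roll and re-arms a reset timer on each update, so ResetLever fires three seconds after the last update.
; ResetLever plays a second timeline to reverse the swing and clears IsLeverActive when finished; the flag is never set or checked here.
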(event `self.LeverAnim`
  (bind (_direction _newtrack_0) (`Timeline|Timeline` :`NewTime` 3.0 :!via `PlayFromStart`)
    (:`Update`
      (`SceneComponent.K2_SetRelativeRotation` (`self.Root`) (`KismetMathLibrary.MakeRotator` (`KismetMathLibrary.Lerp` -45.0 45.0 _newtrack_0)) false false)
      (`KismetSystemLibrary.K2_SetTimerDelegate` (delegate `resetLever`) 3.0))))

(event `resetLever`
  (bind (_direction _newtrack_0) (`Timeline|Timeline_0` :`NewTime` 3.0 :!via `PlayFromStart`)
    (:`Update`
      (`SceneComponent.K2_SetRelativeRotation` (`self.Root`) (`KismetMathLibrary.MakeRotator` (`KismetMathLibrary.Lerp` 45.0 -45.0 _newtrack_0)) false false))
    (:`Finished`
      (set `self.bIsLeverActive` false))))

(fn `UserConstructionScript`)